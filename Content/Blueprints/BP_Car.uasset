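; BP_Car is an actor that drives continuously along a spline path, looping back to the start at the end.
; On BeginPlay it finds a BP_CarSpline actor, then each Tick advances a stored distance and snaps its Scene component to that point's world location and rotation.
; The step adds Speed to DeltaSeconds rather than multiplying them, so movement depends on frame rate.
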(event EventBeginPlay
  (bind _returnvalue (Actor|GetActorOfClass "/Game/Blueprints/BP_CarSpline.BP_CarSpline_C"))
  (Variables|Default|SetSpline _returnvalue))

(event Collision|EventActorBeginOverlap
  (params (OtherActor :type Actor%20Object%20Reference)))

(event EventTick
  (params (DeltaSeconds :type Float%20%28single-precision%29))
  (bind _spline (Variables|Default|GetSpline))
  (bind _scene (Variables|Default|GetScene))
  (bind _spline_component (Variables|/Game/Blueprints/BP_CarSpline.BP_CarSpline_C|GetSpline%20Component _spline))
  (bind _output_get (Variables|Default|SetDistanceAlongSpine (+ (+ DeltaSeconds (Variables|Default|GetSpeed)) (Variables|Default|GetDistanceAlongSpine))))
  (if (>= _output_get (Spline|GetSplineLength _spline_component))
    (Variables|Default|SetDistanceAlongSpine 0.0)
    (else
      (Transformation|SetWorldLocation _scene (Spline|GetLocationatDistanceAlongSpline _spline_component _output_get "World") false false)
      (Transformation|SetWorldRotation _scene (Spline|GetRotationatDistanceAlongSpline _spline_component _output_get "World") false false))))

(fn ConstructionScript)