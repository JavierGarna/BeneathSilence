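; BP_LightingManager produces a periodic lightning flash with thunder by switching a point light between minimum and maximum intensity.
; A looping five-minute timer calls ChangeIntensity, which raises a dimmed light and plays the thunder sound at the actor, or otherwise sets it to minimum.
; Tick watches for maximum intensity and calls the same toggle after a short Delay, ending the flash.
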(event EventBeginPlay
  (Utilities|Time|SetTimerbyFunctionName 0 "ChangeIntensity" 3e+02 true))

(event EventTick
  (params (DeltaSeconds :type Float%20%28single-precision%29))
  (if (== (Variables|/Script/Engine.LightComponentBase|GetIntensity (Variables|Default|GetPointLight)) (Variables|Default|GetMaxIntensity))
    (Utilities|FlowControl|Delay 0.2)
    (CallFunction|ChangeIntensity)))

(fn ConstructionScript)

(fn ChangeIntensity
  (bind _pointlight (Variables|Default|GetPointLight))
  (if (== (Variables|/Script/Engine.LightComponentBase|GetIntensity _pointlight) (Variables|Default|GetMinIntensity))
    (Rendering|Components|Light|SetIntensity _pointlight (Variables|Default|GetMaxIntensity))
    (Audio|SpawnSoundatLocation "/Game/SoundEffects/Thunder.Thunder" (Transformation|GetActorLocation) "0, 0, 0" 1.0 1.0 0.0 0 0)
    (else
      (Rendering|Components|Light|SetIntensity _pointlight (Variables|Default|GetMinIntensity)))))