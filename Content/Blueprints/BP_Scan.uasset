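; BP_Scan is a short-lived actor that emits an expanding scan pulse and a matching noise event in a horror game.
; On BeginPlay it claims a slot index from the HorrorGameInstance, reporting noise and starting only if one is available.
; A timeline writes position, growing radius and late fade into that slot's PC_Scan material parameter collection entries.
; When finished, it releases the slot, resets position and radius, and destroys itself.
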(event Custom|StartScan
  (Rendering|Material|SetVectorParameterValue "/Game/ScanWave/PC_Scan.PC_Scan" (Utilities|Array|Get(acopy) (Variables|Default|GetPositionParameterNames) (Variables|Default|GetScanIndex)) (Math|Conversions|ToLinearColor(Vector) (Transformation|GetActorLocation)) :!class /Script/Engine.KismetMaterialLibrary)
  (Components|Timeline|SetPlayRate (Variables|Default|GetScanExpansion) 0.5)
  (bind _newtrack_0 (Timeline|ScanExpansion Play)
    (:Update
      (Rendering|Material|SetScalarParameterValue "/Game/ScanWave/PC_Scan.PC_Scan" (Utilities|Array|Get(acopy) (Variables|Default|GetRadiusParameterNames) (Variables|Default|GetScanIndex)) (* _newtrack_0 (Variables|Default|GetMax%20Range)) :!class /Script/Engine.KismetMaterialLibrary)
      (Rendering|Material|SetScalarParameterValue "/Game/ScanWave/PC_Scan.PC_Scan" (Utilities|Array|Get(acopy) (Variables|Default|GetFadeParameterValues) (Variables|Default|GetScanIndex)) (- 1.0 (Math|Float|Clamp(Float) (/ (- _newtrack_0 0.8) 0.2))) :!class /Script/Engine.KismetMaterialLibrary))
    (:Finished
      (Class|HorrorGameInstance|RemoveScan (Variables|Default|GetAs%20Horror%20Game%20Instance) (Variables|Default|GetScanIndex))
      (Rendering|Material|SetVectorParameterValue "/Game/ScanWave/PC_Scan.PC_Scan" (Utilities|Array|Get(acopy) (Variables|Default|GetPositionParameterNames) (Variables|Default|GetScanIndex)) (Variables|Default|GetInitialVector) :!class /Script/Engine.KismetMaterialLibrary)
      (Rendering|Material|SetScalarParameterValue "/Game/ScanWave/PC_Scan.PC_Scan" (Utilities|Array|Get(acopy) (Variables|Default|GetRadiusParameterNames) (Variables|Default|GetScanIndex)) 0.0 :!class /Script/Engine.KismetMaterialLibrary)
      (Actor|DestroyActor))))

(event EventBeginPlay
  (bind _ashorror_game_instance (Utilities|Casting|CastToHorrorGameInstance (Game|GetGameInstance)))
  (bind _output_get (Variables|Default|SetAs%20Horror%20Game%20Instance _ashorror_game_instance))
  (bind _returnvalue (Class|HorrorGameInstance|ClaimScan _output_get))
  (bind _output_get_2 (Variables|Default|SetScanIndex _returnvalue))
  (if (!= _output_get_2 -1)
    (Class|AISenseHearing|ReportNoiseEvent (Variables|Default|GetNoise%20Location) (Variables|Default|GetLoudness) (Variables|Actor|GetInstigator) (Variables|Default|GetMax%20Range) "None")
    (CallFunction|StartScan)))

(fn ConstructionScript)