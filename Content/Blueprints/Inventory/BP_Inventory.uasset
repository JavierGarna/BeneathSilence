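; Inventory component that stores item structs in a ten-slot array, shows them in WBP_Inventory, and handles interaction detection and item use.
; Adding or removing an item writes its slot by index and reloads the widget.
; Tick sphere-traces ahead of the player pawn and toggles CanReceiveTraceMessage on hit actors.
; UseItem spawns the first slot's class on the ground below the player, calls UseMessage on it, then clears the slot.
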(event EventBeginPlay
  (bind _returnvalue (UserInterface|CreateWidget "/Game/Blueprints/Inventory/WBP_Inventory.WBP_Inventory_C"))
  (bind _output_get (Variables|Default|SetInventoryWidget _returnvalue))
  (UserInterface|Viewport|AddtoViewport _output_get 0)
  (Utilities|Array|Resize (Variables|Default|GetItems) 10)
  (Default|LoadInventory (Variables|Default|GetInventoryWidget) self))

(event EventTick
  (params (DeltaSeconds :type Float%20%28single-precision%29))
  (CallFunction|InteractionTrace))

(fn AddtoInventory
  (params (ItemID :type Name) (ItemName :type Text) (Icon :type Texture%202D%20Object%20Reference) (ItemClass :type Actor%20Class%20Reference) (Index :type Integer))
  (Utilities|Array|SetArrayElem (Variables|Default|GetItems) Index (Utilities|Struct|MakeST_Item ItemName ItemID Icon ItemClass))
  (Default|LoadInventory (Variables|Default|GetInventoryWidget) self))

(fn RemovefromInventory
  (params (Index :type Integer))
  (Utilities|Array|SetArrayElem (Variables|Default|GetItems) Index (Utilities|Struct|MakeST_Item "" "None" 0))
  (Default|LoadInventory (Variables|Default|GetInventoryWidget) self))

(fn InteractionTrace
  (bind _returnvalue (Game|Player|GetPlayerPawn 0))
  (bind _returnvalue_2 (Transformation|GetActorLocation _returnvalue))
  (bind (_outhit _returnvalue_3) (Collision|SphereTraceByChannel _returnvalue_2 (+ _returnvalue_2 (* (Transformation|GetActorForwardVector _returnvalue) (Variables|Default|GetInteractionRange))) 15.0 "TraceTypeQuery3" false (Utilities|Array|MakeArray (Components|GetOwner)) "None"))
  (if _returnvalue_3
    (if (!= (.HitActor (Collision|BreakHitResult _outhit)) (Variables|Default|GetHit%20Actor))
      (bind _output_get (Variables|Default|SetHit%20Actor (.HitActor (Collision|BreakHitResult _outhit))))
      (Class|BPIInteraction|CanReceiveTrace(Message) _output_get true)
      (else
        (Class|BPIInteraction|CanReceiveTrace(Message) _output_get false)
        (Variables|Default|SetHit%20Actor 0)))))

(fn UseItem
  (bind _returnvalue (Game|Player|GetPlayerPawn 0))
  (bind _returnvalue_2 (Transformation|GetActorLocation _returnvalue))
  (for (_array_element _array_index) (Variables|Default|GetItems)
    (if (== _array_index 0)
      (bind _outhit (Collision|LineTraceByChannel _returnvalue_2 (- _returnvalue_2 "0.000000,0.000000,1000.000000") "TraceTypeQuery1" false 0 "None"))
      (bind _returnvalue_3 (Game|SpawnActorfromClass (.itemclass _array_element) (Math|Transform|MakeTransform (+ (.location (Math|Conversions|ToTransform(Vector) (.location _outhit))) "0.000000,0.000000,5.000000") (.rotation (Math|Conversions|ToTransform(Vector) (.location _outhit))) (.scale (Math|Conversions|ToTransform(Vector) (.location _outhit)))) "AlwaysSpawn" "MultiplyWithRoot" 0 0))
      (Class|BPIInteraction|Use(Message) _returnvalue_3)
      (CallFunction|RemovefromInventory _array_index))))