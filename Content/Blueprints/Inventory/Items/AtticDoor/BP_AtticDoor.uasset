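; BP_AtticDoor is an attic door that unlocks when the player's inventory contains a crowbar.
; Unlock searches the player character's inventory for BP_Crowbar, then plays the door animation once and sets the unlocked flag.
; Once unlocked, Tick lowers a separate static mesh by a fixed, frame-rate-dependent step until it reaches its limit.
; The door renders custom depth, switching stencil value to reflect its locked or unlocked state.
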(event EventBeginPlay
  (bind _door (Variables|Default|GetDoor))
  (|CallParentFunction)
  (Rendering|SetRenderCustomDepth _door true)
  (Rendering|SetCustomDepthStencilValue _door 3)
  (Rendering|SetRenderCustomDepth (Variables|Default|GetStaticMesh) false))

(event Collision|EventActorBeginOverlap
  (params (OtherActor :type Actor%20Object%20Reference))
  (|CallParentFunction OtherActor) ; This node is disabled and will not be called.\nDrag off pins to build functionality.
)

(event EventTick
  (params (DeltaSeconds :type Float%20%28single-precision%29))
  (bind _staticmesh (Variables|Default|GetStaticMesh))
  (|CallParentFunction DeltaSeconds)
  (if (Variables|Default|GetIs%20Unlocked)
    (if (> (.z (Variables|/Script/Engine.SceneComponent|GetRelativeLocation _staticmesh)) -35.0)
      (Transformation|AddRelativeLocation _staticmesh "0.000000,0.000000,-0.300000" false false))))

(fn ConstructionScript
  (|CallParentFunction))

(fn Unlock
  (bind _door (Variables|Default|GetDoor))
  (bind _asbp_player_character (Utilities|Casting|CastToBP_PlayerCharacter (Game|Player|GetPlayerPawn 0)))
  (for _array_element (Variables|/Game/Blueprints/Inventory/BP_Inventory.BP_Inventory_C|GetItems (Variables|/Game/Player/BP_PlayerCharacter.BP_PlayerCharacter_C|GetInventory _asbp_player_character))
    (if (== (.itemclass _array_element) "/Game/Blueprints/Inventory/Items/Crowbar/BP_Crowbar.BP_Crowbar_C")
      (if (not (Variables|Default|GetIs%20Unlocked))
        (Components|Animation|PlayAnimation _door 0 false)
        (Variables|Default|SetIs%20Unlocked true)
        (Rendering|SetCustomDepthStencilValue _door 4)
        (return)))))