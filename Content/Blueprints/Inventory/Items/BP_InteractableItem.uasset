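; Interactable item Blueprint that shows a widget while the player is inside its sphere and supports zoomable, rotatable inspection.
; The construction script copies the static mesh into an inspection mesh 1000 units below, rendered alone by a SceneCapture2D, and enables custom depth stencil on the original.
; Interact unhides that copy, while input events adjust capture FOV within limits and rotate the copy.
; ExitInspectMode is an empty stub.
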(event OnComponentBeginOverlap(Sphere)
  (params (OverlappedComponent :type Primitive%20Component%20Object%20Reference) (OtherActor :type Actor%20Object%20Reference) (OtherComp :type Primitive%20Component%20Object%20Reference) (OtherBodyIndex :type Integer) (bFromSweep :type Boolean) (SweepResult :type Hit%20Result%20Structure%20%28by%20ref%29))
  (Utilities|Casting|CastToBP_PlayerCharacter OtherActor)
  (Rendering|SetVisibility (Variables|Default|GetWidget) true false))

(event OnComponentEndOverlap(Sphere)
  (params (OverlappedComponent :type Primitive%20Component%20Object%20Reference) (OtherActor :type Actor%20Object%20Reference) (OtherComp :type Primitive%20Component%20Object%20Reference) (OtherBodyIndex :type Integer))
  (Utilities|Casting|CastToBP_PlayerCharacter OtherActor)
  (Rendering|SetVisibility (Variables|Default|GetWidget) false false))

(event Custom|UpdateMeshZoom
  (params (Axis :type Float%20%28double-precision%29))
  (bind _scenecapturecomponent2d (Variables|Default|GetSceneCaptureComponent2D))
  (Variables|/Script/Engine.SceneCaptureComponent2D|SetFOVAngle _scenecapturecomponent2d (Math|Float|Clamp(Float) (+ (Variables|/Script/Engine.SceneCaptureComponent2D|GetFOVAngle _scenecapturecomponent2d) (* Axis -3.0)) 4e+01 8e+01)))

(event Custom|UpdateMeshRotation
  (params (Vector2D :type Vector%202D%20Structure))
  (bind _inspectablemesh (Variables|Default|GetInspectableMesh))
  (Transformation|SetRelativeRotation _inspectablemesh (Math|Rotator|CombineRotators (Variables|/Script/Engine.SceneComponent|GetRelativeRotation _inspectablemesh) (Math|Rotator|MakeRotator (* (.y Vector2D) -5.0) (* (.x Vector2D) -5.0) 0.0)) false false))

(event Custom|Exit%20Inspect%20Mode)

(event EventBeginPlay)

(event Collision|EventActorBeginOverlap
  (params (OtherActor :type Actor%20Object%20Reference)))

(event EventTick
  (params (DeltaSeconds :type Float%20%28single-precision%29)))

(event EventInteract
  (Development|SetHiddeninGame (Variables|Default|GetInspectableMesh) false false))

(fn ConstructionScript
  (bind _inspectablemesh (Variables|Default|GetInspectableMesh))
  (bind _staticmesh (Variables|Default|GetStaticMesh))
  (bind _scenecapturecomponent2d (Variables|Default|GetSceneCaptureComponent2D))
  (bind _staticmesh_2 (Variables|Default|GetStaticMesh))
  (bind _relativelocation (Variables|/Script/Engine.SceneComponent|GetRelativeLocation _inspectablemesh))
  (bind _relativelocation_2 (Variables|/Script/Engine.SceneComponent|GetRelativeLocation _scenecapturecomponent2d))
  (Rendering|SceneCapture|ShowOnlyComponent (Variables|Default|GetSceneCaptureComponent2D) _inspectablemesh)
  (Components|StaticMesh|SetStaticMesh _inspectablemesh (Variables|/Script/Engine.StaticMeshComponent|GetStaticMesh _staticmesh))
  (Transformation|SetRelativeTransform _inspectablemesh (Transformation|GetRelativeTransform _staticmesh) false false)
  (Transformation|SetRelativeLocation _inspectablemesh (Math|Vector|MakeVector (.x _relativelocation) (.y _relativelocation) -1e+03) false false)
  (Transformation|SetRelativeLocation _scenecapturecomponent2d (Math|Vector|MakeVector (.x _relativelocation_2) (.y _relativelocation_2) -995.0) false false)
  (Variables|Default|SetItemDefaultTransform (Transformation|GetRelativeTransform (Variables|Default|GetInspectableMesh)))
  (Rendering|SetRenderCustomDepth _staticmesh_2 true)
  (Rendering|SetCustomDepthStencilValue _staticmesh_2 1))