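; BP_Phone is an inventory item pickup that spawns a scan actor when used.
; Interact, gated by a CanInteract flag set through CanReceiveTrace, looks up the "Phone" row in the ItemData table, adds it to the player's inventory and destroys the actor.
; Use spawns BP_Scan at the phone's transform and starts a looping timer that has no function name set.
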(event EventBeginPlay)

(event Collision|EventActorBeginOverlap
  (params (OtherActor :type Actor%20Object%20Reference)))

(event EventTick
  (params (DeltaSeconds :type Float%20%28single-precision%29)))

(event EventInteract
  (if (Variables|Default|GetCan%20Interact)
    (bind _asbp_player_character (Utilities|Casting|CastToBP_PlayerCharacter (Game|Player|GetPlayerPawn 0)))
    (bind _returnvalue (Utilities|GetDataTableRow "/Game/Blueprints/Inventory/ItemData.ItemData" "Phone")
      (:then
        (Default|AddtoInventory (Variables|/Game/Player/BP_PlayerCharacter.BP_PlayerCharacter_C|GetInventory _asbp_player_character) (.itemid _returnvalue) (.itemname _returnvalue) (.icon _returnvalue) (.itemclass _returnvalue))
        (Actor|DestroyActor)))))

(event EventCanReceiveTrace
  (params (CanInteract :type Boolean))
  (Variables|Default|SetCan%20Interact CanInteract))

(event EventUse
  (Utilities|Time|SetTimerbyFunctionName 0 "" 0.2 true)
  (Game|SpawnActorfromClass "/Game/Blueprints/BP_Scan.BP_Scan_C" (Transformation|GetActorTransform) "Undefined" "MultiplyWithRoot" 0 0))

(fn ConstructionScript)