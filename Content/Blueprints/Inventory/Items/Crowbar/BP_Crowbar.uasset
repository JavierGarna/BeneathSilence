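; BP_Crowbar is a crowbar pickup item that the player can inspect and collect.
; On BeginPlay it limits its SceneCapture2D to its own components and sets the pickup prompt; Inspect assigns the crowbar material.
; Interact reads the Crowbar row from the ItemData table, adds it to the player's first empty inventory slot and destroys the actor, which stays if no slot is free.
; The construction script shrinks the inspectable mesh.
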(event EventBeginPlay
  (|CallParentFunction)
  (Rendering|SceneCapture|ShowOnlyActorComponents (Variables|Default|GetSceneCaptureComponent2D) self false)
  (Variables|Default|SetInspectMessage "Press 'E' to pick up crowbar"))

(event Collision|EventActorBeginOverlap
  (params (OtherActor :type Actor%20Object%20Reference))
  (|CallParentFunction OtherActor) ; This node is disabled and will not be called.\nDrag off pins to build functionality.
)

(event EventTick
  (params (DeltaSeconds :type Float%20%28single-precision%29))
  (|CallParentFunction DeltaSeconds) ; This node is disabled and will not be called.\nDrag off pins to build functionality.
)

(event EventInteract
  (bind _asbp_player_character (Utilities|Casting|CastToBP_PlayerCharacter (Game|Player|GetPlayerPawn 0)))
  (bind _returnvalue (Utilities|GetDataTableRow "/Game/Blueprints/Inventory/ItemData.ItemData" "Crowbar")
    (:then
      (Default|GetFirstEmptySlot (Variables|/Game/Player/BP_PlayerCharacter.BP_PlayerCharacter_C|GetInventory _asbp_player_character))
      (if (!= (Variables|/Game/Blueprints/Inventory/BP_Inventory.BP_Inventory_C|GetAvailableSlot (Variables|/Game/Player/BP_PlayerCharacter.BP_PlayerCharacter_C|GetInventory _asbp_player_character)) -1)
        (Default|AddtoInventory (Variables|/Game/Player/BP_PlayerCharacter.BP_PlayerCharacter_C|GetInventory _asbp_player_character) (.itemid _returnvalue) (.itemname _returnvalue) (.icon _returnvalue) (.itemclass _returnvalue) (Variables|/Game/Blueprints/Inventory/BP_Inventory.BP_Inventory_C|GetAvailableSlot (Variables|/Game/Player/BP_PlayerCharacter.BP_PlayerCharacter_C|GetInventory _asbp_player_character)))
        (Actor|DestroyActor)))))

(event EventInspect
  (Variables|Default|SetInspectMaterial "/Game/Blueprints/Inventory/Items/Crowbar/M_Crowbar.M_Crowbar"))

(fn ConstructionScript
  (bind _inspectablemesh (Variables|Default|GetInspectableMesh))
  (bind _returnvalue (Transformation|GetRelativeTransform _inspectablemesh))
  (|CallParentFunction)
  (Transformation|SetRelativeTransform _inspectablemesh (Math|Transform|MakeTransform (.location _returnvalue) (.rotation _returnvalue) "0.020000,0.020000,0.020000") false false))