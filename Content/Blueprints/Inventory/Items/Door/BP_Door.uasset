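; Locked, inspectable door that opens once the player carries its required item.
; Unlock scans the player inventory; a match unlocks the linked Room, switches the custom-depth stencil and removes interaction.
; Each non-matching item checked before a match plays a locked sound and spawns a BP_Scan noise instigated by the level's BP_ItemPawn.
; Once unlocked, Tick swings the mesh to -120 yaw at a frame-rate-dependent speed.
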(event EventBeginPlay
  (bind _staticmesh (Variables|Default|GetStaticMesh))
  (|CallParentFunction)
  (Rendering|SetRenderCustomDepth _staticmesh true)
  (Rendering|SetCustomDepthStencilValue _staticmesh 3)
  (Physics|SetSimulatePhysics _staticmesh false)
  (Variables|Default|SetInspectMessage "The door is locked. I need something to open it")
  (bind _returnvalue (Actor|GetActorOfClass "/Game/Blueprints/Inventory/Items/BP_ItemPawn.BP_ItemPawn_C"))
  (Variables|Default|SetItemPawn _returnvalue))

(event Collision|EventActorBeginOverlap
  (params (OtherActor :type Actor%20Object%20Reference))
  (|CallParentFunction OtherActor) ; This node is disabled and will not be called.\nDrag off pins to build functionality.
)

(event EventTick
  (params (DeltaSeconds :type Float%20%28single-precision%29))
  (bind _staticmesh (Variables|Default|GetStaticMesh))
  (|CallParentFunction DeltaSeconds)
  (if (Variables|Default|GetIsUnlocked)
    (if (> (.yaw (Variables|/Script/Engine.SceneComponent|GetRelativeRotation _staticmesh)) -1.2e+02)
      (Transformation|AddRelativeRotation _staticmesh "0.000000,-1.000000,0.000000" false false))))

(fn ConstructionScript
  (|CallParentFunction))

(fn Unlock
  (if (not (Variables|Default|GetIsUnlocked))
    (bind _asbp_player_character (Utilities|Casting|CastToBP_PlayerCharacter (Game|Player|GetPlayerPawn 0)))
    (for _array_element (Variables|/Game/Blueprints/Inventory/BP_Inventory.BP_Inventory_C|GetItems (Variables|/Game/Player/BP_PlayerCharacter.BP_PlayerCharacter_C|GetInventory _asbp_player_character))
      (if (== (.itemclass _array_element) (Variables|Default|GetRequiredItem))
        (Variables|Default|SetIsUnlocked true)
        (Variables|/Script/BeneathSilence.RoomVolume|SetbIsLocked (Variables|Default|GetRoom) false)
        (Rendering|SetCustomDepthStencilValue (Variables|Default|GetStaticMesh) 4)
        (CallFunction|RemoveInteraction)
        (return)
        (else
          (Audio|PlaySound2D "/Game/SoundEffects/DoorLocked.DoorLocked" 1.0 1.0 0.0 0 0)
          (Game|SpawnActorfromClass "/Game/Blueprints/BP_Scan.BP_Scan_C" (Transformation|GetActorTransform) "Undefined" "MultiplyWithRoot" 0 (Transformation|GetActorLocation) 6e+02 6e+02 (Variables|Default|GetItemPawn)))))))