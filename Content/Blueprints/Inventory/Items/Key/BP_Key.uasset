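; BP_Key is a key pickup item that the player can inspect or collect into their inventory.
; On Interact, it reads the "Key" row from the ItemData table, finds the first empty slot in BP_PlayerCharacter's inventory, adds the item there and destroys itself.
; It stays in the world if no slot is free.
; On Inspect, it sets the inspect material to M_Key.
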(event EventBeginPlay
  (|CallParentFunction) ; This node is disabled and will not be called.\nDrag off pins to build functionality.
)

(event Collision|EventActorBeginOverlap
  (params (OtherActor :type Actor%20Object%20Reference))
  (|CallParentFunction OtherActor) ; This node is disabled and will not be called.\nDrag off pins to build functionality.
)

(event EventTick
  (params (DeltaSeconds :type Float%20%28single-precision%29))
  (|CallParentFunction DeltaSeconds) ; This node is disabled and will not be called.\nDrag off pins to build functionality.
)

(event EventInteract
  (bind _asbp_player_character (Utilities|Casting|CastToBP_PlayerCharacter (Game|Player|GetPlayerPawn 0)))
  (bind _returnvalue (Utilities|GetDataTableRow "/Game/Blueprints/Inventory/ItemData.ItemData" "Key")
    (:then
      (Default|GetFirstEmptySlot (Variables|/Game/Player/BP_PlayerCharacter.BP_PlayerCharacter_C|GetInventory _asbp_player_character))
      (if (!= (Variables|/Game/Blueprints/Inventory/BP_Inventory.BP_Inventory_C|GetAvailableSlot (Variables|/Game/Player/BP_PlayerCharacter.BP_PlayerCharacter_C|GetInventory _asbp_player_character)) -1)
        (Default|AddtoInventory (Variables|/Game/Player/BP_PlayerCharacter.BP_PlayerCharacter_C|GetInventory _asbp_player_character) (.itemid _returnvalue) (.itemname _returnvalue) (.icon _returnvalue) (.itemclass _returnvalue) (Variables|/Game/Blueprints/Inventory/BP_Inventory.BP_Inventory_C|GetAvailableSlot (Variables|/Game/Player/BP_PlayerCharacter.BP_PlayerCharacter_C|GetInventory _asbp_player_character)))
        (Actor|DestroyActor)))))

(event EventInspect
  (Variables|Default|SetInspectMaterial "/Game/Blueprints/Inventory/Items/Key/M_Key.M_Key"))

(fn ConstructionScript
  (|CallParentFunction))