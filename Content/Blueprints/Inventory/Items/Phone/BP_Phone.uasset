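; Phone inventory item that can be picked up, inspected and used as a vibrating noise source.
; Interact copies its ItemData row into the player's first empty inventory slot, then stops audio and destroys the actor.
; Use plays audio and runs a looping timer that spawns BP_Scan with noise parameters, instigated by BP_ItemPawn, until a second timer pauses it.
; Its scene capture renders only the phone itself, and Inspect sets the phone material.
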(event EventBeginPlay
  (Rendering|SceneCapture|ShowOnlyActorComponents (Variables|Default|GetSceneCaptureComponent2D) self false)
  (Variables|Default|SetInspectMessage "Press 'E' to pick up phone")
  (bind _returnvalue (Actor|GetActorOfClass "/Game/Blueprints/Inventory/Items/BP_ItemPawn.BP_ItemPawn_C"))
  (Variables|Default|SetItemPawn _returnvalue))

(event Collision|EventActorBeginOverlap
  (params (OtherActor :type Actor%20Object%20Reference)))

(event EventTick
  (params (DeltaSeconds :type Float%20%28single-precision%29)))

(event EventInteract
  (bind _asbp_player_character (Utilities|Casting|CastToBP_PlayerCharacter (Game|Player|GetPlayerPawn 0)))
  (bind _returnvalue (Utilities|GetDataTableRow "/Game/Blueprints/Inventory/ItemData.ItemData" "Phone")
    (:then
      (Default|GetFirstEmptySlot (Variables|/Game/Player/BP_PlayerCharacter.BP_PlayerCharacter_C|GetInventory _asbp_player_character))
      (if (!= (Variables|/Game/Blueprints/Inventory/BP_Inventory.BP_Inventory_C|GetAvailableSlot (Variables|/Game/Player/BP_PlayerCharacter.BP_PlayerCharacter_C|GetInventory _asbp_player_character)) -1)
        (Default|AddtoInventory (Variables|/Game/Player/BP_PlayerCharacter.BP_PlayerCharacter_C|GetInventory _asbp_player_character) (.itemid _returnvalue) (.itemname _returnvalue) (.icon _returnvalue) (.itemclass _returnvalue) (Variables|/Game/Blueprints/Inventory/BP_Inventory.BP_Inventory_C|GetAvailableSlot (Variables|/Game/Player/BP_PlayerCharacter.BP_PlayerCharacter_C|GetInventory _asbp_player_character)))
        (CallFunction|TurnonOffAudio false)
        (Actor|DestroyActor)))))

(event EventCanReceiveTrace
  (params (CanInteract :type Boolean))
  (Variables|Default|SetCan%20Interact CanInteract))

(event EventUse
  (CallFunction|TurnonOffAudio true)
  (Utilities|Time|SetTimerbyFunctionName 0 "Vibration" 0.5 true)
  (Utilities|Time|SetTimerbyFunctionName 0 "StopVibration" 11.0))

(event EventInspect
  (Variables|Default|SetInspectMaterial "/Game/Blueprints/Inventory/Items/Phone/M_Phone.M_Phone"))

(fn ConstructionScript)

(fn Vibration
  (Game|SpawnActorfromClass "/Game/Blueprints/BP_Scan.BP_Scan_C" (Transformation|GetActorTransform) "Undefined" "MultiplyWithRoot" 0 (Transformation|GetActorLocation) 2e+03 2e+03 (Variables|Default|GetItemPawn)))

(fn StopVibration
  (Class|KismetSystemLibrary|PauseTimer 0 "Vibration"))

(fn TurnonOffAudio
  (params (TurnOn :type Boolean))
  (bind _audio (Variables|Default|GetAudio))
  (if TurnOn
    (Audio|Components|Audio|Play _audio 0.0)
    (else
      (Audio|Components|Audio|Stop _audio))))