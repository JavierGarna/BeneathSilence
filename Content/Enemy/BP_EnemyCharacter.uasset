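; Enemy character that gives the monster an audio cue matching its AI state and renders its mesh to custom depth with a stencil value.
; Each tick it reads the CurrentState enum from its controller's blackboard and, on a change, calls UpdateEnemySound.
; That function restarts the audio component with breathing for Search and Run Away, a laugh for Investigate, or a scream for Chase.
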(event EventBeginPlay
  (bind _mesh (Variables|Character|GetMesh))
  (Rendering|SetRenderCustomDepth _mesh true)
  (Rendering|SetCustomDepthStencilValue _mesh 2)
  (CallFunction|UpdateEnemySound "NewEnumerator1"))

(event Collision|EventActorBeginOverlap
  (params (OtherActor :type Actor%20Object%20Reference)))

(event EventTick
  (params (DeltaSeconds :type Float%20%28single-precision%29))
  (bind _returnvalue (Pawn|GetController))
  (bind _currentstate (Variables|Default|GetCurrentState))
  (bind _returnvalue_2 (AI|GetBlackboard _returnvalue))
  (bind _returnvalue_3 (Class|BlackboardComponent|GetValueasEnum _returnvalue_2 _currentstate))
  (if (!= _returnvalue_3 (Variables|Default|GetLastState))
    (bind _output_get (Variables|Default|SetLastState _returnvalue_3))
    (CallFunction|UpdateEnemySound (Utilities|Enum|ByteToEnumCurrentState _output_get))))

(fn ConstructionScript)

(fn UpdateEnemySound
  (params (CurrentState :type CurrentState%20Enum :default "NewEnumerator1"))
  (bind _audio (Variables|Default|GetAudio))
  (bind _audio_2 (Variables|Default|GetAudio))
  (bind _audio_3 (Variables|Default|GetAudio))
  (switch Utilities|FlowControl|Switch|SwitchonCurrentState CurrentState
    (:NewEnumerator1
      (Audio|Components|Audio|Stop _audio_2 :!label _label)
      (Audio|Components|Audio|SetSound _audio_2 "/Game/Enemy/Source/monsterbreathing.monsterbreathing")
      (Audio|Components|Audio|Play _audio_2 0.0))
    (:NewEnumerator2
      (Audio|Components|Audio|Stop _audio)
      (Audio|Components|Audio|SetSound _audio "/Game/Enemy/Source/MonsterLaugh.MonsterLaugh")
      (Audio|Components|Audio|Play _audio 0.0))
    (:NewEnumerator3
      (Audio|Components|Audio|Stop _audio_3)
      (Audio|Components|Audio|SetSound _audio_3 "/Game/Enemy/Source/MonsterScream.MonsterScream")
      (Audio|Components|Audio|Play _audio_3 0.0))
    (:NewEnumerator4
      (goto _label))))