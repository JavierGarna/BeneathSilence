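; Enemy manager Blueprint that trains or runs neural-network enemy agents using the Learning Agents plugin.
; BeginPlay builds the interactor, policy, critic, training environment, shared-memory trainer process and PPO trainer on the LearningAgentsManager.
; RunInference switches Tick between policy inference and PPO training; when off, it also reinitializes the networks at startup.
; The trainer process and PPO trainer are created in both modes.
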(event EventBeginPlay
  (bind _trainer_process_settings (Variables|Default|GetTrainer%20Process%20Settings))
  (bind _shared_memory_settings (Variables|Default|GetShared%20Memory%20Settings))
  (bind _run_inference (Variables|Default|GetRun%20Inference))
  (bind _returnvalue (not _run_inference))
  (Utilities|FlowControl|Sequence
    (:then_0
      (bind _returnvalue_2 (Class|LearningAgentsInteractor|MakeInteractor (Variables|Default|GetLearningAgentsManager) "/Script/BeneathSilence.EnemyInteractor" "EnemyInteractor"))
      (Variables|Default|SetInteractor _returnvalue_2))
    (:then_1
      (bind _returnvalue_3 (Class|LearningAgentsPolicy|MakePolicy (Variables|Default|GetLearningAgentsManager) (Variables|Default|GetInteractor) "/Script/LearningAgents.LearningAgentsPolicy" "EnemyPolicy" "/Game/Enemy/Learning/NN_EnemyEncoder.NN_EnemyEncoder" "/Game/Enemy/Learning/NN_EnemyPolicy.NN_EnemyPolicy" "/Game/Enemy/Learning/NN_EnemyDecoder.NN_EnemyDecoder" _returnvalue _returnvalue _returnvalue (Variables|Default|GetPolicy%20Settings) 3456))
      (Variables|Default|SetPolicy _returnvalue_3))
    (:then_2
      (bind _returnvalue_4 (Class|LearningAgentsCritic|MakeCritic (Variables|Default|GetLearningAgentsManager) (Variables|Default|GetInteractor) (Variables|Default|GetPolicy) "/Script/LearningAgents.LearningAgentsCritic" "EnemyCritic" 0 (not (Variables|Default|GetRun%20Inference)) (Variables|Default|GetCritic%20Settings) 1234))
      (Variables|Default|SetCritic _returnvalue_4))
    (:then_3
      (bind _returnvalue_5 (Class|LearningAgentsTrainingEnvironment|MakeTrainingEnvironment (Variables|Default|GetLearningAgentsManager) "/Script/BeneathSilence.EnemyTrainingEnv" "TrainingEnvironment"))
      (Variables|Default|SetTraining%20Env _returnvalue_5))
    (:then_4
      (bind _returnvalue_6 (Class|LearningAgentsCommunicatorLibrary|SpawnSharedMemoryTrainingProcess _trainer_process_settings _shared_memory_settings))
      (bind _returnvalue_7 (Class|LearningAgentsCommunicatorLibrary|MakeSharedMemoryCommunicator _returnvalue_6 _trainer_process_settings _shared_memory_settings))
      (Variables|Default|SetCommunicator _returnvalue_7))
    (:then_5
      (bind _returnvalue_8 (Class|LearningAgentsPPOTrainer|MakePPOTrainer (Variables|Default|GetLearningAgentsManager) (Variables|Default|GetInteractor) (Variables|Default|GetTraining%20Env) (Variables|Default|GetPolicy) (Variables|Default|GetCritic) (Variables|Default|GetCommunicator) "/Script/LearningAgentsTraining.LearningAgentsPPOTrainer" "PPOTrainer" (Variables|Default|GetTrainer%20Settings)))
      (Variables|Default|SetPPOTrainer _returnvalue_8))))

(event Collision|EventActorBeginOverlap
  (params (OtherActor :type Actor%20Object%20Reference)))

(event EventTick
  (params (DeltaSeconds :type Float%20%28single-precision%29))
  (if (Variables|Default|GetRun%20Inference)
    (Class|LearningAgentsPolicy|RunInference (Variables|Default|GetPolicy) 0.0)
    (else
      (Class|LearningAgentsPPOTrainer|RunTraining (Variables|Default|GetPPOTrainer) (Variables|Default|GetTrainer%20Training%20Settings) (Variables|Default|GetTraining%20Game%20Settings) true true))))

(fn ConstructionScript)