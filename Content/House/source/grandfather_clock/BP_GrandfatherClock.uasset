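; Grandfather clock that ticks and periodically chimes, emitting noise scans through BP_Scan with the item pawn as instigator.
; While the enemy's blackboard points to the clock's room, Tick advances a timer against a random threshold re-rolled each frame, then swaps ticking for a MetaSound chime.
; The MetaSound's watched OnChime output triggers Chime, whose looping timer spawns a burst of scans with one beat skipped.
; Ticking resumes when chime audio finishes.
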(event Custom|OnAudioFinished_Event
  (Audio|Components|Audio|Play (Variables|Default|GetClockSound) 0.0)
  (Variables|Default|SetIsChiming false))

(event Custom|ChimeTimerTick
  (bind _output_get (Variables|Default|SetChimeIndex (+ (Variables|Default|GetChimeIndex) 1)))
  (switch int _output_get
    (:0
      _)
    (:1
      _)
    (:2
      _)
    (:3
      _)
    (:5
      _)
    (:6
      _)
    (:7
      _)
    (:8
      _))
  (Game|SpawnActorfromClass "/Game/Blueprints/BP_Scan.BP_Scan_C" (Transformation|GetActorTransform) "Undefined" "MultiplyWithRoot" 0 (+ (* (Transformation|GetActorForwardVector) 5e+01) (Transformation|GetActorLocation)) 2e+03 2e+03 (Variables|Default|GetItemPawn))
  (if (>= (Variables|Default|GetChimeIndex) 8.0)
    (Utilities|Time|ClearandInvalidateTimerbyHandle (Variables|Default|GetChimeTimerHandle))))

(event EventBeginPlay
  (bind _returnvalue (Audio|SpawnSound2D "/Game/SoundEffects/ClockTicking.ClockTicking" 1.0 1.0 0.0 0 false false))
  (Variables|Default|SetClockSound _returnvalue)
  (bind _returnvalue_2 (Actor|GetActorOfClass "/Game/Enemy/BP_EnemyCharacter.BP_EnemyCharacter_C"))
  (Variables|Default|SetEnemyCharacter _returnvalue_2)
  (bind _returnvalue_3 (Actor|GetActorOfClass "/Game/Blueprints/Inventory/Items/BP_ItemPawn.BP_ItemPawn_C"))
  (Variables|Default|SetItemPawn _returnvalue_3))

(event EventTick
  (params (DeltaSeconds :type Float%20%28single-precision%29))
  (if (Variables|Default|GetChimeStarted)
    (CallFunction|Chime)
    (bind _output_get (Variables|Default|SetChimeTimer (+ (Variables|Default|GetChimeTimer) DeltaSeconds) :!label _label))
    (if (> _output_get (Math|Random|RandomFloatinRange 1e+01 3e+01))
      (Variables|Default|SetChimeTimer 0.0)
      (if (not (Variables|Default|GetIsChiming))
        (Variables|Default|SetIsChiming true)
        (Audio|Components|Audio|Stop (Variables|Default|GetClockSound))
        (bind _returnvalue (Audio|SpawnSound2D "/Game/SoundEffects/MS_ClockChimes.MS_ClockChimes" 1.0 1.0 0.0 0))
        (bind _returnvalue_2 (Class|MetasoundGeneratorHandle|CreateMetaSoundGeneratorHandle _returnvalue))
        (MetaSoundOutput|WatchOutput _returnvalue_2 "OnChime" (EventDispatchers|CreateEvent :!event BPGrandfatherClockAutoGenFunc) "None" "None" :!class /Script/MetasoundEngine.MetasoundGeneratorHandle)
        (EventDispatchers|AssignOnAudioFinished _returnvalue (delegate Custom|OnAudioFinished_Event))))
    (elif (== (AI|Components|Blackboard|GetValueasObject (AI|GetBlackboard (Variables|Default|GetEnemyCharacter)) (Variables|Default|GetKey%20Name)) (Variables|Default|GetClockRoom))
      (goto _label))))

(fn ConstructionScript)

(fn BPGrandfatherClockAutoGenFunc
  (params (OutputName :type Name) (Output :type Meta%20Sound%20Output%20Structure%20%28by%20ref%29))
  (Variables|Default|SetChimeStarted true)
  (return))

(fn Chime
  (Variables|Default|SetChimeStarted false)
  (Variables|Default|SetChimeIndex 0)
  (Game|SpawnActorfromClass "/Game/Blueprints/BP_Scan.BP_Scan_C" (Transformation|GetActorTransform) "Undefined" "MultiplyWithRoot" 0 (+ (* (Transformation|GetActorForwardVector) 5e+01) (Transformation|GetActorLocation)) 2e+03 2e+03 (Variables|Default|GetItemPawn))
  (bind _returnvalue (Utilities|Time|SetTimerbyEvent (EventDispatchers|CreateEvent :!event Custom|ChimeTimerTick) 0.5 true))
  (Variables|Default|SetChimeTimerHandle _returnvalue))