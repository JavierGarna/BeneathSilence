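; Car prop whose alarm goes off when the player enters its trigger box, playing a sound, flashing lights and making loud noise.
; A looping timer repeatedly spawns a noise actor ahead of the car, instigated by the level's BP_ItemPawn, and blinks four point lights.
; Tick stops and re-arms the alarm after a few cycles.
; The alarm flag is set before the player cast, so any other overlapping actor leaves it stuck on.
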(event OnComponentBeginOverlap(Box)
  (params (OverlappedComponent :type Primitive%20Component%20Object%20Reference) (OtherActor :type Actor%20Object%20Reference) (OtherComp :type Primitive%20Component%20Object%20Reference) (OtherBodyIndex :type Integer) (bFromSweep :type Boolean) (SweepResult :type Hit%20Result%20Structure%20%28by%20ref%29))
  (if (not (Variables|Default|GetisAlarmOn))
    (Variables|Default|SetisAlarmOn true)
    (Utilities|Casting|CastToBP_PlayerCharacter OtherActor)
    (Audio|SpawnSoundatLocation "/Game/SoundEffects/CarAlarm.CarAlarm" (Transformation|GetActorLocation) "0, 0, 0" 1.0 1.0 0.0 0 0)
    (Game|SpawnActorfromClass "/Game/Blueprints/BP_Scan.BP_Scan_C" (Transformation|GetActorTransform) "Undefined" "MultiplyWithRoot" 0 (+ (* (Transformation|GetActorForwardVector) 3.5e+02) (Transformation|GetActorLocation)) 2e+03 0.0 (Variables|Default|GetItemPawn))
    (CallFunction|TurnonLights)
    (bind _returnvalue (Utilities|Time|SetTimerbyFunctionName 0 "Alarm" 1.5 true))
    (Variables|Default|SetAlarmTimer _returnvalue)))

(event Custom|TurnOffLights
  (Rendering|SetVisibility (Variables|Default|GetPointLight1) false false))

(event Custom|TurnOnLights
  (Rendering|SetVisibility (Variables|Default|GetPointLight1) true false)
  (Utilities|Time|SetTimerbyEvent (delegate Custom|TurnOffLights) 0.5))

(event EventBeginPlay
  (bind _returnvalue (Actor|GetActorOfClass "/Game/Blueprints/Inventory/Items/BP_ItemPawn.BP_ItemPawn_C"))
  (Variables|Default|SetItemPawn _returnvalue))

(event Collision|EventActorBeginOverlap
  (params (OtherActor :type Actor%20Object%20Reference)))

(event EventTick
  (params (DeltaSeconds :type Float%20%28single-precision%29))
  (if (>= (Variables|Default|GetAlarmCounter) 3)
    (Variables|Default|SetAlarmCounter 0)
    (Utilities|Time|ClearandInvalidateTimerbyHandle (Variables|Default|GetAlarmTimer))
    (Variables|Default|SetisAlarmOn false)))

(fn ConstructionScript)

(fn Alarm
  (Game|SpawnActorfromClass "/Game/Blueprints/BP_Scan.BP_Scan_C" (Transformation|GetActorTransform) "Undefined" "MultiplyWithRoot" 0 (+ (* (Transformation|GetActorForwardVector) 3.5e+02) (Transformation|GetActorLocation)) 2e+03 0.0 (Variables|Default|GetItemPawn))
  (CallFunction|TurnonLights)
  (Variables|Default|SetAlarmCounter (+ (Variables|Default|GetAlarmCounter) 1)))