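; Player character Blueprint handling interaction, item inspection, inventory hotkeys, pause menu and win/loss screens polled from the game mode on Tick.
; A forward trace unlocks doors or opens a 3D inspection overlay, swapping input contexts for rotate, zoom and accept/reject.
; Footsteps spawn noise-carrying BP_Scan actors at bone positions.
; BeginPlay registers the character with Learning Agents managers tagged PlayerILManager.
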(event Custom|ExitInspectionMode
  (bind _returnvalue (PlayerController|LocalPlayerSubsystems|GetEnhancedInputLocalPlayerSubsystem))
  (bind _3dwidget (Variables|Default|Get3DWidget))
  (if (Widget|IsVisible _3dwidget)
    (Widget|RemovefromParent _3dwidget)
    (Class|EnhancedInputSubsystemInterface|ClearAllMappings _returnvalue)
    (Input|AddMappingContext _returnvalue "/Game/Player/Input/IMC_Player.IMC_Player" 0 "(bIgnoreAllPressedKeysUntilRelease=True,bForceImmediately=False,bNotifyUserSettings=False)")
    (if (Variables|Default|GetInspectionAnswer)
      (Class|BPIInteraction|Interact(Message) (Variables|Default|GetHitItem)))))

(event Custom|UpdateInputMappingContext
  (bind _returnvalue (PlayerController|LocalPlayerSubsystems|GetEnhancedInputLocalPlayerSubsystem))
  (Utilities|IsValid _returnvalue
    (:Is%20Valid
      (Class|EnhancedInputSubsystemInterface|ClearAllMappings _returnvalue)
      (Input|AddMappingContext _returnvalue "/Game/Player/Input/InspectionsIA/IMC_Inspection.IMC_Inspection" 0 "(bIgnoreAllPressedKeysUntilRelease=True,bForceImmediately=False,bNotifyUserSettings=False)"))))

(event Input|EnhancedActionEvents|EnhancedInputActionIA_InventorySlot
  (params (ActionValue :type Boolean) (ElapsedSeconds :type Float%20%28double-precision%29) (TriggeredSeconds :type Float%20%28double-precision%29) (InputAction :type Input%20Action%20Object%20Reference :default "/Game/Player/Input/IA_InventorySlot.IA_InventorySlot"))
  (:Completed
    (if (not (Widget|IsVisible (Variables|Default|Get3DWidget)))
      (Default|UseItem (Variables|Default|GetInventory) (Variables|Default|GetLastInventoryKeyPressed)))))

(event Input|EnhancedActionEvents|EnhancedInputActionIA_MouseMove
  (params (ActionValue :type Vector%202D%20Structure) (ElapsedSeconds :type Float%20%28double-precision%29) (TriggeredSeconds :type Float%20%28double-precision%29) (InputAction :type Input%20Action%20Object%20Reference :default "/Game/Player/Input/InspectionsIA/IA_MouseMove.IA_MouseMove"))
  (if (Variables|Default|GetLeftClickActive)
    (Default|UpdateMeshRotation (Variables|Default|GetInteractableItem) ActionValue)))

(event Input|EnhancedActionEvents|EnhancedInputActionIA_LeftMouseClick
  (params (ActionValue :type Boolean) (ElapsedSeconds :type Float%20%28double-precision%29) (TriggeredSeconds :type Float%20%28double-precision%29) (InputAction :type Input%20Action%20Object%20Reference :default "/Game/Player/Input/InspectionsIA/IA_LeftMouseClick.IA_LeftMouseClick"))
  (:Started
    (Variables|Default|SetLeftClickActive true))
  (:Completed
    (Variables|Default|SetLeftClickActive false)))

(event Input|EnhancedActionEvents|EnhancedInputActionIA_Accept
  (params (ActionValue :type Boolean) (ElapsedSeconds :type Float%20%28double-precision%29) (TriggeredSeconds :type Float%20%28double-precision%29) (InputAction :type Input%20Action%20Object%20Reference :default "/Game/Player/Input/InspectionsIA/IA_Accept.IA_Accept"))
  (Variables|Default|SetInspectionAnswer true)
  (CallFunction|ExitInspectionMode))

(event Input|EnhancedActionEvents|EnhancedInputActionIA_MouseWheel
  (params (ActionValue :type Float%20%28double-precision%29) (ElapsedSeconds :type Float%20%28double-precision%29) (TriggeredSeconds :type Float%20%28double-precision%29) (InputAction :type Input%20Action%20Object%20Reference :default "/Game/Player/Input/InspectionsIA/IA_MouseWheel.IA_MouseWheel"))
  (Default|UpdateMeshZoom (Variables|Default|GetInteractableItem) ActionValue))

(event Input|EnhancedActionEvents|EnhancedInputActionIA_Pause
  (params (ActionValue :type Boolean) (ElapsedSeconds :type Float%20%28double-precision%29) (TriggeredSeconds :type Float%20%28double-precision%29) (InputAction :type Input%20Action%20Object%20Reference :default "/Game/Player/Input/IA_Pause.IA_Pause"))
  (:Started
    (CallFunction|TogglePause)))

(event Input|EnhancedActionEvents|EnhancedInputActionIA_Reject
  (params (ActionValue :type Boolean) (ElapsedSeconds :type Float%20%28double-precision%29) (TriggeredSeconds :type Float%20%28double-precision%29) (InputAction :type Input%20Action%20Object%20Reference :default "/Game/Player/Input/InspectionsIA/IA_Reject.IA_Reject"))
  (Variables|Default|SetInspectionAnswer false)
  (CallFunction|ExitInspectionMode))

(event Input|EnhancedActionEvents|EnhancedInputActionIA_Interact
  (params (ActionValue :type Boolean) (ElapsedSeconds :type Float%20%28double-precision%29) (TriggeredSeconds :type Float%20%28double-precision%29) (InputAction :type Input%20Action%20Object%20Reference :default "/Game/Player/Input/IA_Interact.IA_Interact"))
  (CallFunction|CheckInteraction))

(event EventBeginPlay
  (bind _returnvalue (UserInterface|CreateWidget "/Game/Blueprints/Inventory/Items/WB_3DOverlay.WB_3DOverlay_C"))
  (Variables|Default|Set3DWidget _returnvalue)
  (bind _outactors (Actor|GetAllActorswithTag "PlayerILManager"))
  (for _array_element _outactors
    (Utilities|IsValid (Actor|GetComponentbyClass _array_element "/Script/LearningAgents.LearningAgentsManager")
      (:Is%20Valid
        (Class|LearningAgentsManager|AddAgent (Actor|GetComponentbyClass _array_element "/Script/LearningAgents.LearningAgentsManager") self)
        (Variables|Default|SetFoundManager true))))
  (if (not (Variables|Default|GetFoundManager))
    (Development|PrintString "RecordingManager not found")))

(event EventTick
  (params (DeltaSeconds :type Float%20%28single-precision%29))
  (bind _asmain_game_mode_base (Utilities|Casting|CastToMainGameModeBase (Game|GetGameMode)))
  (if (Class|MainGameModeBase|GetHasWon _asmain_game_mode_base)
    (bind _returnvalue (UserInterface|CreateWidget "/Game/UI/Win.Win_C"))
    (UserInterface|Viewport|AddtoViewport _returnvalue 0)
    (bind _asmain_player_controller (Utilities|Casting|CastToMainPlayerController (Game|GetPlayerController 0) :!label _label))
    (Variables|/Script/Engine.PlayerController|SetbShowMouseCursor _asmain_player_controller true)
    (Game|SetGamePaused true)
    (elif (Class|MainGameModeBase|GetHasLost _asmain_game_mode_base)
      (bind _returnvalue_2 (UserInterface|CreateWidget "/Game/UI/Lost.Lost_C"))
      (UserInterface|Viewport|AddtoViewport _returnvalue_2 0)
      (goto _label))))

(event Input|KeyboardEvents|1
  (params (Key :type Key%20Structure :default "None"))
  (:Pressed
    (Variables|Default|SetLastInventoryKeyPressed 0)))

(event Input|KeyboardEvents|2
  (params (Key :type Key%20Structure :default "None"))
  (:Pressed
    (Variables|Default|SetLastInventoryKeyPressed 1)))

(event Input|KeyboardEvents|3
  (params (Key :type Key%20Structure :default "None"))
  (:Pressed
    (Variables|Default|SetLastInventoryKeyPressed 2)))

(event Input|KeyboardEvents|4
  (params (Key :type Key%20Structure :default "None"))
  (:Pressed
    (Variables|Default|SetLastInventoryKeyPressed 3)))

(event Input|KeyboardEvents|5
  (params (Key :type Key%20Structure :default "None"))
  (:Pressed
    (Variables|Default|SetLastInventoryKeyPressed 4)))

(fn ConstructionScript)

(fn HandleFootstepScan
  (params (Bone%20Name :type Name) (Loudness :type Float%20%28double-precision%29) (Max%20Range :type Float%20%28double-precision%29))
  (Game|SpawnActorfromClass "/Game/Blueprints/BP_Scan.BP_Scan_C" (Transformation|GetBoneTransform (Variables|Character|GetMesh) Bone%20Name "RTS_World") "Undefined" "MultiplyWithRoot" 0 (Transformation|GetActorLocation) Loudness Max%20Range self))

(fn CheckInteraction
  (bind _returnvalue (Game|GetPlayerController 0))
  (bind _returnvalue_2 (Transformation|GetActorLocation))
  (bind (_outhit _returnvalue_3) (Collision|LineTraceByChannel _returnvalue_2 (+ _returnvalue_2 (* (Transformation|GetActorForwardVector) 100)) "TraceTypeQuery3" false 0 "None"))
  (bind _output_get (Variables|Default|SetHitItem (.HitActor (Collision|BreakHitResult _outhit))))
  (bind _asbp_interactable_item (Utilities|Casting|CastToBP_InteractableItem _output_get))
  (bind _output_get_2 (Variables|Default|SetInteractableItem _asbp_interactable_item))
  (if _returnvalue_3
    (bind _asbp_door (Utilities|Casting|CastToBP_Door _output_get_2)
      (:then
        (Default|Unlock _asbp_door))
      (:CastFailed
        (bind _asbp_attic_door (Utilities|Casting|CastToBP_AtticDoor _output_get_2)
          (:then
            (Default|Unlock _asbp_attic_door))
          (:CastFailed
            (Default|Inspect _output_get_2)
            (Variables|Default|SetInspect%20Material (Variables|/Game/Blueprints/Inventory/Items/BP_InteractableItem.BP_InteractableItem_C|GetInspectMaterial _output_get_2))
            (UserInterface|Viewport|AddtoViewport (Variables|Default|Get3DWidget) 0)
            (CallFunction|UpdateInputMappingContext)
            (Variables|/Script/Engine.PlayerController|SetbShowMouseCursor _returnvalue true)
            (Input|SetInputModeGameandUI _returnvalue 0 "DoNotLock" true false)))))))

(fn TogglePause
  (bind _returnvalue (Game|GetPlayerController 0))
  (bind _returnvalue_2 (Game|GetPlayerController 0))
  (if (Variables|Default|GetIsPaused)
    (Variables|Default|SetIsPaused false)
    (Widget|RemovefromParent (Variables|Default|GetPauseMenuRef))
    (Input|SetInputModeGameOnly _returnvalue_2 false)
    (Variables|/Script/Engine.PlayerController|SetbShowMouseCursor _returnvalue_2 false)
    (else
      (bind _returnvalue_3 (UserInterface|CreateWidget "/Game/UI/PauseMenu.PauseMenu_C"))
      (Variables|Default|SetPauseMenuRef _returnvalue_3)
      (UserInterface|Viewport|AddtoViewport _returnvalue_3 0)
      (Variables|Default|SetIsPaused true)
      (Input|SetInputModeUIOnly _returnvalue _returnvalue_3 "DoNotLock" false)
      (Variables|/Script/Engine.PlayerController|SetbShowMouseCursor _returnvalue true))))