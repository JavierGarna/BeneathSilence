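; Learning Agents manager actor that trains a policy to imitate the player from the REC_Player recording.
; BeginPlay caches the player and builds the interactor, policy, shared-memory trainer process and communicator, and imitation trainer.
; Tick only runs policy inference when RunInference is set.
; Otherwise, with a valid trainer, each Tick runs training, saves the policy, encoder and decoder networks to NN_Player assets, then runs inference.
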(event EventBeginPlay
  (bind _trainer_process_settings (Variables|Default|GetTrainer%20Process%20Settings))
  (bind _shared_memory_settings (Variables|Default|GetShared%20Memory%20Settings))
  (Utilities|FlowControl|Sequence
    (:then_0
      (bind _returnvalue (Actor|GetActorOfClass "/Game/Player/BP_PlayerCharacter.BP_PlayerCharacter_C"))
      (Variables|Default|SetPlayer _returnvalue))
    (:then_1
      (bind _returnvalue_2 (Class|LearningAgentsInteractor|MakeInteractor (Variables|Default|GetLearningAgentsManager) "/Script/BeneathSilence.PlayerInteractor" "Interactor"))
      (Variables|Default|SetInteractor _returnvalue_2))
    (:then_2
      (bind _returnvalue_3 (Class|LearningAgentsPolicy|MakePolicy (Variables|Default|GetLearningAgentsManager) (Variables|Default|GetInteractor) "/Script/LearningAgents.LearningAgentsPolicy" "Policy" (Variables|Default|GetEncoder%20Neural%20Network%20Asset) (Variables|Default|GetPolicy%20Neural%20Network%20Asset) (Variables|Default|GetDecoder%20Neural%20Network%20Asset) true true true (Variables|Default|GetPolicy%20Settings) 1234))
      (Variables|Default|SetPolicy _returnvalue_3))
    (:then_3
      (bind _returnvalue_4 (Class|LearningAgentsCommunicatorLibrary|SpawnSharedMemoryTrainingProcess _trainer_process_settings _shared_memory_settings))
      (bind _returnvalue_5 (Class|LearningAgentsCommunicatorLibrary|MakeSharedMemoryCommunicator _returnvalue_4 _trainer_process_settings _shared_memory_settings))
      (Variables|Default|SetCommunicator _returnvalue_5))
    (:then_4
      (bind _returnvalue_6 (Class|LearningAgentsImitationTrainer|MakeImitationTrainer (Variables|Default|GetLearningAgentsManager) (Variables|Default|GetInteractor) (Variables|Default|GetPolicy) (Variables|Default|GetCommunicator) "/Script/LearningAgentsTraining.LearningAgentsImitationTrainer" "ImitationTrainer"))
      (Variables|Default|SetImitation%20Trainer _returnvalue_6))))

(event EventTick
  (params (DeltaSeconds :type Float%20%28single-precision%29))
  (bind _imitation_trainer (Variables|Default|GetImitation%20Trainer))
  (bind _policy (Variables|Default|GetPolicy))
  (if (Variables|Default|GetbRunInference)
    (Class|LearningAgentsPolicy|RunInference (Variables|Default|GetPolicy) 1.0)
    (else
      (Utilities|IsValid _imitation_trainer
        (:Is%20Valid
          (Class|LearningAgentsImitationTrainer|RunTraining _imitation_trainer "/Game/PlayerImitator/REC_Player.REC_Player" (Variables|Default|GetImitation%20Trainer%20Settings) (Variables|Default|GetImitation%20Trainer%20Training%20Settings) (Variables|Default|GetImitation%20Trainer%20Path%20Settings))
          (Class|LearningAgentsNeuralNetwork|SaveNetworktoAsset (Class|LearningAgentsPolicy|GetPolicyNetworkAsset _policy) "/Game/PlayerImitator/NN_PlayerPolicy.NN_PlayerPolicy")
          (Class|LearningAgentsNeuralNetwork|SaveNetworktoAsset (Class|LearningAgentsPolicy|GetEncoderNetworkAsset _policy) "/Game/PlayerImitator/NN_PlayerEncoder.NN_PlayerEncoder")
          (Class|LearningAgentsNeuralNetwork|SaveNetworktoAsset (Class|LearningAgentsPolicy|GetDecoderNetworkAsset _policy) "/Game/PlayerImitator/NN_PlayerDecoder.NN_PlayerDecoder")
          (Class|LearningAgentsPolicy|RunInference _policy 1.0))))))

(fn ConstructionScript)