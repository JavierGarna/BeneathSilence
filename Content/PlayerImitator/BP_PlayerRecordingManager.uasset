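; Learning Agents manager Blueprint that records player behavior to the REC_Player asset, part of the PlayerImitator setup.
; BeginPlay caches the BP_PlayerCharacter, builds an interactor, controller and recorder on the LearningAgentsManager, then starts recording.
; Each Tick runs the PlayerAIController and adds the resulting experience to the recorder, and EndPlay ends the recording.
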(event EventBeginPlay
  (Utilities|FlowControl|Sequence
    (:then_0
      (bind _returnvalue (Actor|GetActorOfClass "/Game/Player/BP_PlayerCharacter.BP_PlayerCharacter_C"))
      (Variables|Default|SetPlayer _returnvalue))
    (:then_1
      (bind _returnvalue_2 (Class|LearningAgentsInteractor|MakeInteractor (Variables|Default|GetLearningAgentsManager) "/Script/BeneathSilence.PlayerInteractor" "Interactor"))
      (Variables|Default|SetInteractor _returnvalue_2))
    (:then_2
      (bind _returnvalue_3 (Class|LearningAgentsController|MakeController (Variables|Default|GetLearningAgentsManager) (Variables|Default|GetInteractor) "/Script/BeneathSilence.PlayerAIController" "Controller"))
      (Variables|Default|SetController _returnvalue_3))
    (:then_3
      (bind _returnvalue_4 (Class|LearningAgentsRecorder|MakeRecorder (Variables|Default|GetLearningAgentsManager) (Variables|Default|GetInteractor) "/Script/LearningAgentsTraining.LearningAgentsRecorder" "Recorder" (Variables|Default|GetRecorder%20Path%20Settings) "/Game/PlayerImitator/REC_Player.REC_Player" true))
      (Variables|Default|SetRecorder _returnvalue_4))
    (:then_4
      (Class|LearningAgentsRecorder|BeginRecording (Variables|Default|GetRecorder)))))

(event EventTick
  (params (DeltaSeconds :type Float%20%28single-precision%29))
  (Class|LearningAgentsController|RunController (Variables|Default|GetController))
  (Class|LearningAgentsRecorder|AddExperience (Variables|Default|GetRecorder)))

(event EventEndPlay
  (params (EndPlayReason :type EEndPlayReason%20Enum :default "Destroyed"))
  (Class|LearningAgentsRecorder|EndRecording (Variables|Default|GetRecorder)))

(fn ConstructionScript)